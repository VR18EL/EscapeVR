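; Interactive shelf cabinet prop that the player opens and closes with the E key.
; TriggerBoxR overlap enables or disables input from player controller 0, without checking which actor overlapped.
; E toggles IsClose, playing the matching skeletal mesh animation and a sound at world origin, and is ignored mid-animation.
; Tick polls the animation state and hides the UI component through SetUI while it plays.
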(event OnComponentBeginOverlap(TriggerBoxR)
  (params (OverlappedComponent :type Primitive%20Component%20Object%20Reference) (OtherActor :type Actor%20Object%20Reference) (OtherComp :type Primitive%20Component%20Object%20Reference) (OtherBodyIndex :type Integer) (bFromSweep :type Boolean) (SweepResult :type Hit%20Result%20Structure%20%28by%20ref%29))
  (Input|EnableInput (Game|GetPlayerController 0)))

(event OnComponentEndOverlap(TriggerBoxR)
  (params (OverlappedComponent :type Primitive%20Component%20Object%20Reference) (OtherActor :type Actor%20Object%20Reference) (OtherComp :type Primitive%20Component%20Object%20Reference) (OtherBodyIndex :type Integer))
  (Input|DisableInput (Game|GetPlayerController 0)))

(event EventBeginPlay)

(event Collision|EventActorBeginOverlap
  (params (OtherActor :type Actor%20Object%20Reference)))

(event EventTick
  (params (DeltaSeconds :type Float%20%28single-precision%29))
  (if (Audio|Components|Audio|IsPlaying (Variables|Default|GetSKM_ShelfCabinet))
    (CallFunction|SetUI true)
    (else
      (CallFunction|SetUI false))))

(event Input|KeyboardEvents|E
  (params (Key :type Key%20Structure))
  (bind _skm_shelfcabinet (Variables|Default|GetSKM_ShelfCabinet))
  (:Pressed
    (if (not (Audio|Components|Audio|IsPlaying _skm_shelfcabinet))
      (if (Variables|Default|GetIsClose)
        (Components|Animation|PlayAnimation _skm_shelfcabinet "/Game/CH/KTInteractionPropVol2/Animation/ANIM_ShelfCabinet_Open.ANIM_ShelfCabinet_Open" false)
        (Variables|Default|SetIsClose false)
        (Audio|PlaySoundatLocation "/Game/CH/KTInteractionPropVol2/Sound/Sound_StorageCabinets_Open.Sound_StorageCabinets_Open" "0, 0, 0" "0, 0, 0" 1.0 1.0 0.0 0 0 0 0)
        (else
          (Components|Animation|PlayAnimation _skm_shelfcabinet "/Game/CH/KTInteractionPropVol2/Animation/ANIM_ShelfCabinet_Close.ANIM_ShelfCabinet_Close" false)
          (Variables|Default|SetIsClose true)
          (Audio|PlaySoundatLocation "/Game/CH/KTInteractionPropVol2/Sound/Sound_StorageCabinets_Close.Sound_StorageCabinets_Close" "0, 0, 0" "0, 0, 0" 1.0 1.0 0.0 0 0 0 0))))))

(fn ConstructionScript)

(fn SetUI
  (params (Hidden :type Boolean))
  (Development|SetHiddeninGame (Variables|Default|GetUI) Hidden false))